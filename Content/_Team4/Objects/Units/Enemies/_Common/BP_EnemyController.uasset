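; Shared AI controller for enemies derived from BBP_Enemy.
; On possess it runs the enemy's own behavior tree, copies its attack distance, attack interval and strafe radius (as fall-back radius) into the blackboard, then sets the initial state, or prints an error if no tree is assigned.
; Helper functions set the current target and get or set the enemy state through blackboard keys.
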(event `self.ReceivePossess`
  (params (PossessedPawn :type "Pawn Object Reference"))
  (bind _asbbp_enemy (cast `/Game/_Team4/Objects/Units/Enemies/_Common/Graphics/BBP_Enemy` PossessedPawn))
  (bind _behaviortree (`/Game/_Team4/Objects/Units/Enemies/_Common/Graphics/BBP_Enemy.BehaviorTree` _asbbp_enemy)
    (:`then`
      (`self.RunBehaviorTree` _behaviortree)
      (`self.SetupBlackboardVariables` _asbbp_enemy)
      (`self.SetCurrentState` "NewEnumerator0"))
    (:`else`
      (`KismetSystemLibrary.PrintString` "No valid Behavior Tree in enemy found!!!"))))

(fn `GetCurrentState`
  (returns (CurrentState :type "/Game/_Team4/Objects/Units/Enemies/_Common/Enums/E_EnemyState Enum"))
  (return (cast `/Game/_Team4/Objects/Units/Enemies/_Common/Enums/E_EnemyState` (`BlackboardComponent.GetValueAsEnum` (`self.Blackboard`) (`self.CurrentStateKey`)))))

(fn `SetCurrentState`
  (params (`New State` :type "/Game/_Team4/Objects/Units/Enemies/_Common/Enums/E_EnemyState Enum" :default "NewEnumerator0"))
  (`BlackboardComponent.SetValueAsEnum` (`self.Blackboard`) (`self.CurrentStateKey`) `New State`))

(fn `SetCurrentTarget`
  (params (`New Target` :type "Actor Object Reference"))
  (`BlackboardComponent.SetValueAsObject` (`self.Blackboard`) (`self.TargetKey`) `New Target`))

(fn `SetupBlackboardVariables`
  (params (PossessedEnemy :type "/Game/_Team4/Objects/Units/Enemies/_Common/Graphics/BBP_Enemy Object Reference"))
  (bind _blackboard (`self.Blackboard`))
  (`BlackboardComponent.SetValueAsFloat` _blackboard (`self.MinAttackDistanceKey`) (`/Game/_Team4/Objects/Units/Enemies/_Common/Graphics/BBP_Enemy.MinAttackDistance` PossessedEnemy))
  (`BlackboardComponent.SetValueAsFloat` _blackboard (`self.AttackTimeIntervalKey`) (`/Game/_Team4/Objects/Units/Enemies/_Common/Graphics/BBP_Enemy.AttackTimeInterval` PossessedEnemy))
  (`BlackboardComponent.SetValueAsFloat` _blackboard (`self.FallBackRadiusKey`) (`/Game/_Team4/Objects/Units/Enemies/_Common/Graphics/BBP_Enemy.StrafeRadius` PossessedEnemy)))

(fn `UserConstructionScript`)